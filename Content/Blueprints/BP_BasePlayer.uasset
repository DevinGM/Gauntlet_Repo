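; BP_BasePlayer is a base player Blueprint that handles movement and projectile shooting, with input mappings for two players.
; Both players' axis inputs are bound in the same graph and add movement along the control rotation's yaw-based forward and right vectors.
; Only the P1 attack is bound, spawning BP_Projectile at the ProjectileSpawnPos transform.
; A note says shots should follow the last movement input, but the graph does not track it.
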(event Input|ActionEvents|InputActionAttack_P1
  (params (Key :type Key%20Structure :default "None"))
  ;[1 1 1] Shooting Mechanic (needs to fire in direction of last movement input)
  (:Pressed
    (Game|SpawnActorfromClass "/Game/Blueprints/BP_Projectile.BP_Projectile_C" (Transformation|GetWorldTransform (Variables|Default|GetProjectileSpawnPos)) "Undefined" 0 0)))

(event Input|AxisEvents|InputAxisLeftRight_P1
  (params (AxisValue :type Float%20%28single-precision%29))
  ;[1 1 1] Movement Controls
  (Pawn|Input|AddMovementInput (Math|Vector|GetRightVector (Math|Rotator|MakeRotator 0.0 0.0 (.yaw (Pawn|GetControlRotation :!class /Script/Engine.Pawn)))) AxisValue false))

(event Input|AxisEvents|InputAxisLeftRight_P2
  (params (AxisValue :type Float%20%28single-precision%29))
  ;[1 1 1] Movement Controls
  (Pawn|Input|AddMovementInput (Math|Vector|GetRightVector (Math|Rotator|MakeRotator 0.0 0.0 (.yaw (Pawn|GetControlRotation :!class /Script/Engine.Pawn)))) AxisValue false))

(event Input|AxisEvents|InputAxisUpDown_P1
  (params (AxisValue :type Float%20%28single-precision%29))
  ;[1 1 1] Movement Controls
  (Pawn|Input|AddMovementInput (Math|Vector|GetForwardVector (Math|Rotator|MakeRotator 0.0 0.0 (.yaw (Pawn|GetControlRotation :!class /Script/Engine.Pawn)))) AxisValue false))

(event Input|AxisEvents|InputAxisUpDown_P2
  (params (AxisValue :type Float%20%28single-precision%29))
  ;[1 1 1] Movement Controls
  (Pawn|Input|AddMovementInput (Math|Vector|GetForwardVector (Math|Rotator|MakeRotator 0.0 0.0 (.yaw (Pawn|GetControlRotation :!class /Script/Engine.Pawn)))) AxisValue false))

(fn ConstructionScript)