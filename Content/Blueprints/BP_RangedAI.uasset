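; Ranged enemy AI that chases the player and fires projectiles on sight.
; PawnSensing sightings start an AIMoveTo toward the player, turn the enemy to face a seen BP_BasePlayer, and spawn BP_Projectile from ProjectileSpawnPos.
; A CanAttack flag with a short delay limits fire rate.
; PlayerPos is read only at BeginPlay, before MoveToPlayer assigns PlayerRef, which also serves as the move's target actor.
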(event OnSeePawn(PawnSensing)
  (params (Pawn :type Pawn%20Object%20Reference))
  ;[1 1 1] Shoot Function, enemy will fire projectiles at player when player enters sight range.
  (Utilities|FlowControl|Sequence
    (:then_0
      ;[0 0.4125 1] Follow Player
      (CallFunction|MovetoPlayer))
    (:then_1
      (bind _asbp_base_player (Utilities|Casting|CastToBP_BasePlayer Pawn))
      (Transformation|SetActorRotation (Math|Rotator|FindLookatRotation (Transformation|GetActorLocation) (Transformation|GetActorLocation _asbp_base_player)))
      (if (Variables|Default|GetCanAttack)
        (Game|SpawnActorfromClass "/Game/Blueprints/BP_Projectile.BP_Projectile_C" (Transformation|GetWorldTransform (Variables|Default|GetProjectileSpawnPos)) "Undefined" 0 0)
        (Variables|Default|SetCanAttack false)
        (Utilities|FlowControl|Delay 0.5)
        (Variables|Default|SetCanAttack true)))))

(event Custom|MoveToPlayer
  ;[0 0.4125 1] Follow Player
  ;;[1 1 1] Follow Movement
  (bind _asbp_base_player (Utilities|Casting|CastToBP_BasePlayer (Game|GetPlayerCharacter 0)))
  (bind _output_get (Variables|Default|SetPlayerRef _asbp_base_player))
  (AI|AIMoveTo self (Variables|Default|GetPlayerPos) _output_get 5.0 false))

(event Custom|GetPlayerPos
  ;[0 0.4125 1] Follow Player
  ;;[1 1 1] Get Player Position
  (Variables|Default|SetPlayerPos (Transformation|GetActorLocation (Variables|Default|GetPlayerRef))))

(event EventBeginPlay
  ;[0 0.4125 1] Follow Player
  ;;[1 1 1] Update Player Position
  (CallFunction|GetPlayerPos))

(fn ConstructionScript)