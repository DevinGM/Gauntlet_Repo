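; Enemy AI pawn that chases the player on sight and deals damage on contact.
; PawnSensing sets IsSeeingPlayer, which is never cleared here, and triggers FollowPlayer to run AIMoveTo toward player character 0, regardless of which pawn was seen.
; Overlapping an actor that casts to PlayerParent calls DealDamageToPlayer with the Damage variable.
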(event OnSeePawn(PawnSensing)
  (params (Pawn :type Pawn%20Object%20Reference))
  ;[1 1 1] Basic Chase Movement (follows player as soon as entity sees player controller)
  (Variables|Logic|SetIsSeeingPlayer true)
  (CallFunction|FollowPlayer))

(event Custom|FollowPlayer
  ;[1 1 1] Basic Chase Movement (follows player as soon as entity sees player controller)
  (if (Variables|Logic|GetIsSeeingPlayer)
    (AI|AIMoveTo self "0, 0, 0" (Game|GetPlayerCharacter 0) 5.0 false)))

(event Collision|EventActorBeginOverlap
  (params (OtherActor :type Actor%20Object%20Reference))
  (bind _asplayer_parent (Utilities|Casting|CastToPlayerParent OtherActor))
  (Class|PlayerParent|DealDamagetoPlayer _asplayer_parent (Variables|Stats|GetDamage)))

(fn ConstructionScript)