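; Ranged enemy AI that turns toward the player and fires projectiles when its PawnSensing component sees them.
; Each sighting calls MoveToPlayer, which issues AIMoveTo toward player controller 0, or toward itself when within a short range of PlayerRef.
; It then snaps rotation to the seen BP_BasePlayer and spawns BP_Projectile at ProjectileSpawnPos.
; A CanAttack flag and Delay throttle the fire rate.
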(event OnSeePawn(PawnSensing)
  (params (Pawn :type Pawn%20Object%20Reference))
  ;[1 1 1] Shoot Function, enemy will fire projectiles at player when player enters sight range.
  (Utilities|FlowControl|Sequence
    (:then_0
      (CallFunction|MovetoPlayer))
    (:then_1
      (bind _asbp_base_player (Utilities|Casting|CastToBP_BasePlayer Pawn))
      (Transformation|SetActorRotation (Math|Rotator|FindLookatRotation (Transformation|GetActorLocation) (Transformation|GetActorLocation _asbp_base_player)))
      (if (Variables|Default|GetCanAttack)
        (Game|SpawnActorfromClass "/Game/Blueprints/BP_Projectile.BP_Projectile_C" (Transformation|GetWorldTransform (Variables|Default|GetProjectileSpawnPos)) "Undefined" 0 0)
        (Variables|Default|SetCanAttack false)
        (Utilities|FlowControl|Delay 0.5)
        (Variables|Default|SetCanAttack true)))))

(event Custom|MoveToPlayer
  (if (>= (Transformation|GetDistanceTo (Variables|Default|GetPlayerRef)) 1e+02)
    (AI|AIMoveTo self "0, 0, 0" (Game|GetPlayerController 0) 5.0 false
      (:then
        _))
    (else
      (AI|AIMoveTo self "0, 0, 0" self 5.0 true
        (:then
          _))))
  (Utilities|FlowControl|Delay 0.1))

(fn ConstructionScript)