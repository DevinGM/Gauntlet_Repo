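; BP_EnemyAI is an enemy that chases the player once its PawnSensing component sees a pawn.
; Any sighting sets IsSeeingPlayer, which is never cleared here, and calls FollowPlayer to issue an AI MoveTo toward player character 0, without checking which pawn was seen.
; Capsule overlaps only print a debug message for non-PlayerParent actors; player contact does nothing and Damage is unused.
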(event OnComponentBeginOverlap(CapsuleComponent)
  (params (OverlappedComponent :type Primitive%20Component%20Object%20Reference) (OtherActor :type Actor%20Object%20Reference) (OtherComp :type Primitive%20Component%20Object%20Reference) (OtherBodyIndex :type Integer) (bFromSweep :type Boolean) (SweepResult :type Hit%20Result%20Structure%20%28by%20ref%29))
  (Utilities|Casting|CastToPlayerParent OtherActor
    (:CastFailed
      (Development|PrintString "Enemy collided with not a player"))))

(event OnSeePawn(PawnSensing)
  (params (Pawn :type Pawn%20Object%20Reference))
  ;[1 1 1] Basic Chase Movement (follows player as soon as entity sees player controller)
  (Variables|Logic|SetIsSeeingPlayer true)
  (CallFunction|FollowPlayer))

(event Custom|FollowPlayer
  ;[1 1 1] Basic Chase Movement (follows player as soon as entity sees player controller)
  (if (Variables|Logic|GetIsSeeingPlayer)
    (AI|AIMoveTo self "0, 0, 0" (Game|GetPlayerCharacter 0) 5.0 false)))

(fn ConstructionScript)